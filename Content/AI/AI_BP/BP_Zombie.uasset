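; BP_Zombie is an AI zombie pawn that spots the third-person player and damages them at close range.
; Pawn sensing sets the "Spotted?" Blackboard bool on seeing the player, and nothing here clears it.
; The AIAttack event runs a short forward line trace with persistent debug drawing and applies damage if it hits the player.
; The attack montage and an experimental sphere trace are disconnected, so attacks play no animation.
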(event OnSeePawn(PawnSensing)
  (params (Pawn :type Pawn%20Object%20Reference))
  ;[1 1 1] When the pawn sensing detects the player than it will get the blackboard bool value and change the has seen bool value to true. Knows which blackboard value by the name passed into the make litteral node blueprint
  (Utilities|Casting|CastToBP_ThirdPersonCharacter Pawn)
  (AI|Components|Blackboard|SetValueasBool (AI|GetBlackboard (AI|GetAIController self)) (Utilities|Name|MakeLiteralName "Spotted?") true))

(event Custom|AIAttack
  (bind _returnvalue (Transformation|GetActorLocation))
  ;[1 1 1] Determines how to detect the player character with the pawn array in the line trace for objects, then checks if its the thirpersoncharacter and if it is then play the attack anime montage and deal damage to the player
  ;;[0.03103 1 0.9801] Experminenting for best trace object node
  (bind (_outhit _returnvalue_2) (Collision|LineTraceForObjects _returnvalue (+ _returnvalue (* (Math|Vector|GetForwardVector (Transformation|GetActorRotation)) 2.5e+02)) (Utilities|Array|MakeArray "ObjectTypeQuery3") false 0 "Persistent"))
  (if _returnvalue_2
    (Utilities|Casting|CastToBP_ThirdPersonCharacter (.HitActor (Collision|BreakHitResult _outhit)))
    (Game|Damage|ApplyDamage (.HitActor (Collision|BreakHitResult _outhit)) 5e+01 0 0)))

(event EventBeginPlay)

(event Collision|EventActorBeginOverlap
  (params (OtherActor :type Actor%20Object%20Reference)))

(event EventTick
  (params (DeltaSeconds :type Float%20%28single-precision%29)))

(fn ConstructionScript)